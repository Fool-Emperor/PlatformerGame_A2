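; Platformer enemy turret that fires BP_Bullet actors from its firing point and can optionally turn to face the player.
; BeginPlay starts either single-shot or scatter-shot fire, each a self-calling event looped through a firing delay.
; Scatter shot spawns a burst of bullets with randomized yaw spread.
; When LookAtPlayer is set, Tick rotates the turret body using a look-at built from X and Y positions only.
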(event Custom|OneShot
  ;[0.15 0.15 0.15 0.5] One Shot
  (Game|SpawnActorfromClass "/Game/_Platformer/Blueprints/BP_Bullet.BP_Bullet_C" (Transformation|GetSocketTransform (Variables|Default|GetFiring%20Point) "None" "RTS_World") "AlwaysSpawn" "MultiplyWithRoot" 0 0)
  (Utilities|FlowControl|Delay (Variables|Default|GetFiringDelay))
  (CallFunction|OneShot))

(event Custom|ScatterShot
  (bind _firing_point (Variables|Default|GetFiring%20Point))
  (bind _returnvalue (Transformation|GetSocketTransform _firing_point "None" "RTS_World"))
  ;[0.15 0.15 0.15 0.5] Scatter Shot
  (for _index (range 0 4)
    (Game|SpawnActorfromClass "/Game/_Platformer/Blueprints/BP_Bullet.BP_Bullet_C" (Math|Transform|MakeTransform (.location _returnvalue) (Math|Rotator|MakeRotator (.roll (.rotation _returnvalue)) (.pitch (.rotation _returnvalue)) (+ (.yaw (.rotation _returnvalue)) (Math|Random|RandomFloatinRange -3e+01 3e+01)))) "AlwaysSpawn" "MultiplyWithRoot" 0 0))
  (Utilities|FlowControl|Delay (Variables|Default|GetFiringDelay))
  (CallFunction|ScatterShot))

(event EventBeginPlay
  ;[0.15 0.15 0.15 0.5] Set Up Firing Shot
  (if (Variables|Default|GetUseScatterShot)
    (CallFunction|ScatterShot)
    (else
      (CallFunction|OneShot))))

(event Collision|EventActorBeginOverlap
  (params (OtherActor :type Actor%20Object%20Reference))
  ;[0.15 0.15 0.15 0.5] Set Up Firing Shot
)

(event EventTick
  (params (DeltaSeconds :type Float%20%28single-precision%29))
  (bind _returnvalue (Transformation|GetActorLocation))
  (bind _returnvalue_2 (Game|Player|GetPlayerPawn 0))
  (bind _returnvalue_3 (Transformation|GetActorLocation _returnvalue_2))
  ;[0.15 0.15 0.15 0.5] Rotate Turret
  (if (Variables|Default|GetLookAtPlayer)
    (Transformation|SetRelativeRotation (Variables|Default|GetSM_Turret_Body) (Math|Rotator|FindLookatRotation (Math|Vector|MakeVector (.x _returnvalue) (.y _returnvalue) 0.0) (Math|Vector|MakeVector (.x _returnvalue_3) (.y _returnvalue_3) 0.0)) false false)))

(fn ConstructionScript)