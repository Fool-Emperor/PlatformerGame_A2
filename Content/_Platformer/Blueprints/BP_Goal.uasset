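; BP_Goal is a platformer goal actor that stays hidden and non-collidable until the player has collected enough coins.
; BeginPlay caches the player pawn as a BP_ThirdPersonCharacter reference.
; Every Tick compares that character's collected coin count against CoinGoal and uses the result to set SMGoal visibility and actor collision.
; The file contains no logic for reaching the goal, as its overlap event is empty.
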(event EventBeginPlay
  ;[0.15 0.15 0.15 0.5] Get Player Character
  (bind _asbp_third_person_character (Utilities|Casting|CastToBP_ThirdPersonCharacter (Game|Player|GetPlayerPawn 0)))
  (Variables|Default|SetPlayer%20Reference _asbp_third_person_character))

(event Collision|EventActorBeginOverlap
  (params (OtherActor :type Actor%20Object%20Reference)))

(event EventTick
  (params (DeltaSeconds :type Float%20%28single-precision%29))
  ;[0.15 0.15 0.15 0.5] Set Goal Visibility
  (bind _output_get (Variables|Default|SetCoinGoalMet (>= (Variables|/Game/_Platformer/Blueprints/BP_ThirdPersonCharacter.BP_ThirdPersonCharacter_C|GetNumberOfCoinsCollected (Variables|Default|GetPlayer%20Reference)) (Variables|Default|GetCoinGoal))))
  (Rendering|SetVisibility (Variables|Default|GetSM_Goal) _output_get _output_get)
  (Collision|SetActorEnableCollision _output_get))

(fn ConstructionScript)