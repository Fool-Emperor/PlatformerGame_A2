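; Platformer platform that vanishes after the player stands on it continuously for a set lifetime, then reappears after a delay.
; Overlap events on a detection component flag the player's presence, and Tick accumulates time while flagged, resetting it otherwise.
; At the lifetime limit the actor hides and disables collision, then after a Delay restores visibility, collision and the transform saved at BeginPlay.
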(event OnComponentBeginOverlap(PlayerPlatformDetection)
  (params (OverlappedComponent :type Primitive%20Component%20Object%20Reference) (OtherActor :type Actor%20Object%20Reference) (OtherComp :type Primitive%20Component%20Object%20Reference) (OtherBodyIndex :type Integer) (bFromSweep :type Boolean) (SweepResult :type Hit%20Result%20Structure%20%28by%20ref%29))
  ;[0.15 0.15 0.15 0.5] Collider Check
  (if (== OtherActor (Game|Player|GetPlayerPawn 0))
    (Utilities|FlowControl|Sequence
      (:then_0
        (Variables|Default|SetIsPlayerOnPlatform true)))))

(event OnComponentEndOverlap(PlayerPlatformDetection)
  (params (OverlappedComponent :type Primitive%20Component%20Object%20Reference) (OtherActor :type Actor%20Object%20Reference) (OtherComp :type Primitive%20Component%20Object%20Reference) (OtherBodyIndex :type Integer))
  ;[0.15 0.15 0.15 0.5] Collider Check
  (if (== OtherActor (Game|Player|GetPlayerPawn 0))
    (Utilities|FlowControl|Sequence
      (:then_0
        (Variables|Default|SetIsPlayerOnPlatform false)))))

(event Custom|ReturnToDefault
  ;[0.15 0.15 0.15 0.5] Return to Default
  (Transformation|SetWorldTransform (Variables|Default|GetDefaultSceneRoot) (Variables|Default|GetStartTransform) false true)
  (Variables|Default|SetTimeOnPlatform 0.0)
  (Rendering|SetActorHiddenInGame false)
  (Collision|SetActorEnableCollision true))

(event EventBeginPlay
  ;[0.15 0.15 0.15 0.5] Set Start Position, Rotation, and Scale
  (Variables|Default|SetStartTransform (Transformation|GetActorTransform)))

(event EventTick
  (params (DeltaSeconds :type Float%20%28single-precision%29))
  ;[0.15 0.15 0.15 0.5] Set Timer for Platform
  (if (Variables|Default|GetIsPlayerOnPlatform)
    (bind _output_get (Variables|Default|SetTimeOnPlatform (+ (Variables|Default|GetTimeOnPlatform) DeltaSeconds)))
    (Utilities|FlowControl|Sequence
      (:then_0
        ;[0.15 0.15 0.15 0.5] Check if Timer has reached Platform's Lifetime
        (if (>= (Variables|Default|GetTimeOnPlatform) (Variables|Default|GetPlatformLifetime))
          ;[0.15 0.15 0.15 0.5] Hide and Disable Platform
          (Rendering|SetActorHiddenInGame true)
          (Collision|SetActorEnableCollision false)
          (Utilities|FlowControl|Delay (Variables|Default|GetTimeInvisible))
          (CallFunction|ReturntoDefault))))
    (else
      (Variables|Default|SetTimeOnPlatform 0.0))))

(fn ConstructionScript)